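; BP_SpikeTrap is a trap that raises spikes and damages the first-person player.
; Overlapping the activation collision plays a timeline that lifts the spike mesh, then reverses it, while a separate damage collision calls DamageUpdate on the player.
; It binds to a player trap dispatcher; a matching trap type permanently disables it by switching off both collisions and destroying the spike mesh.
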(event OnComponentBeginOverlap(DamageColl)
  (params (OverlappedComponent :type Primitive%20Component%20Object%20Reference) (OtherActor :type Actor%20Object%20Reference) (OtherComp :type Primitive%20Component%20Object%20Reference) (OtherBodyIndex :type Integer) (bFromSweep :type Boolean) (SweepResult :type Hit%20Result%20Structure%20%28by%20ref%29))
  (if (== OtherActor (Variables|Default|GetAs%20BP%20First%20Person%20Character))
    (Default|DamageUpdate (Variables|Default|GetAs%20BP%20First%20Person%20Character) 25.0)))

(event OnComponentBeginOverlap(ActivationColl)
  (params (OverlappedComponent :type Primitive%20Component%20Object%20Reference) (OtherActor :type Actor%20Object%20Reference) (OtherComp :type Primitive%20Component%20Object%20Reference) (OtherBodyIndex :type Integer) (bFromSweep :type Boolean) (SweepResult :type Hit%20Result%20Structure%20%28by%20ref%29))
  (bind _sm_spike (Variables|Default|GetSM_Spike))
  (bind _relativelocation (Variables|/Script/Engine.SceneComponent|GetRelativeLocation _sm_spike))
  (if (== OtherActor (Variables|Default|GetAs%20BP%20First%20Person%20Character))
    (bind (_direction _movementtrack) (Timeline|SpikeMovementTimeline Play)
      (:Update
        (Transformation|SetRelativeLocation (Variables|Default|GetSM_Spike) (Math|Vector|MakeVector (.x _relativelocation) (.y _relativelocation) (Math|Float|Lerp 0.0 1e+02 _movementtrack)) false false)
        (if true
          _))
      (:Finished
        (switch Utilities|FlowControl|Switch|SwitchonETimelineDirection _direction
          (:Forward
            (Timeline|SpikeMovementTimeline ReverseFromEnd)))))))

(event Custom|DP_Trap_Event
  (params (TrapType :type TrapType%20Enum :default "NewEnumerator0"))
  (if (Utilities|Enum|Equal(Enum) TrapType (Variables|Default|GetTrapType))
    (Transformation|SetRelativeLocation (Variables|Default|GetSM_Spike) "0, 0, 0" false false)
    (Collision|SetCollisionEnabled (Variables|Default|GetDamageColl) "NoCollision")
    (Components|DestroyComponent (Variables|Default|GetSM_Spike))))

(event EventBeginPlay
  (bind _asbp_first_person_character (Utilities|Casting|CastToBP_FirstPersonCharacter (Game|GetPlayerCharacter 0)))
  (bind _output_get (Variables|Default|SetAs%20BP%20First%20Person%20Character _asbp_first_person_character))
  (EventDispatchers|BindEventtoDPTrap _output_get (delegate Custom|DP_Trap_Event)))

(fn ConstructionScript)